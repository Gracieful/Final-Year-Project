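; BP_OSC_LookUp moves BPSphereMove actors using right-eye gaze values received over OSC.
; On BeginPlay it starts an OSC server and binds message handling, which wildcard-matches the eye look up, in and out addresses.
; Each match calls SetLocation from the last-read floats: in minus out scales to Y, up scales to Z, and X stays zero.
; A look-down branch exists but is disconnected.
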(event Custom|OnMsgReceived
  (params (Message :type OSC%20Message%20Structure%20%28by%20ref%29) (IPAddress :type String) (Port :type Integer))
  ;[1 1 1] OSC
  (bind _returnvalue (Class|OSCManager|GetOSCMessageAddress Message))
  (bind _returnvalue_2 (Class|OSCManager|GetOSCAddressFullPath _returnvalue))
  (Utilities|FlowControl|Sequence
    (:then_1
      ;[1 1 1] Gets LookUp
      (if (Class|KismetStringLibrary|MatchesWildcard _returnvalue_2 "/f1:eyeLookUpRight" "IgnoreCase")
        (bind _value (Class|OSCManager|GetFloat Message))
        ;[1 1 1] Ball Movement
        (bind _outactors (Actor|GetAllActorsOfClass (Variables|Default|GetBP_Sphere_move) :!label _label))
        (Default|SetLocation _outactors 0.0 (+ (* (stale _value_2) (Variables|Default|GetMultiplyY)) (* (stale _value_3) (* (Variables|Default|GetMultiplyY) -1.0))) (+ 0.0 (* _value (Variables|Default|GetMultiplyZ))))))
    (:then_2
      ;[1 1 1] Gets Look In
      (if (Class|KismetStringLibrary|MatchesWildcard _returnvalue_2 "/f1:eyeLookInRight" "IgnoreCase")
        (bind _value_2 (Class|OSCManager|GetFloat Message (Math|Integer|%(Integer) 0 1)))
        (goto _label)))
    (:then_3
      ;[1 1 1] Gets Look Out
      (if (Class|KismetStringLibrary|MatchesWildcard _returnvalue_2 "/f1:eyeLookOutRight" "IgnoreCase")
        (bind _value_3 (Class|OSCManager|GetFloat Message))
        (goto _label)))))

(event EventBeginPlay
  ;[1 1 1] OSC
  (bind _returnvalue (Class|OSCManager|CreateOSCServer (Variables|Default|GetIPAddress) (Variables|Default|GetPort%20ID) false true (Variables|Default|GetServer%20Name_1) 0))
  (bind _output_get (Variables|Default|SetLookUp _returnvalue))
  (EventDispatchers|AssignOnOscMessageReceived _output_get (delegate Custom|OnMsgReceived)))

(fn ConstructionScript)